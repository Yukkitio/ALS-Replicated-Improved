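; Data-driven weapon actor that takes its weapon name and owner from the first BPI_Interact actor overlapping its sphere.
; UpdateValues loads mesh, sound, effects and stats from Weapon_Table by WeaponName, on construction and RepNotify.
; FireON fires once or opens a Tick gate for automatic fire, with DoOnce and Delay limiting rate.
; Fire traces from camera, re-traces from muzzle socket to catch obstructions, then applies effects, impulse and fixed damage.
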(event OnComponentBeginOverlap(Sphere)
  (params (OverlappedComponent :type Primitive%20Component%20Object%20Reference) (OtherActor :type Actor%20Object%20Reference) (OtherComp :type Primitive%20Component%20Object%20Reference) (OtherBodyIndex :type Integer) (bFromSweep :type Boolean) (SweepResult :type Hit%20Result%20Structure%20%28by%20ref%29))
  (if (Utilities|DoesObjectImplementInterface OtherActor "/Game/Inventory/BPI_Interact.BPI_Interact_C")
    (bind _weaponname (Class|BPIInteract|GetWeaponName(Message) OtherActor))
    (Variables|Default|SetWeaponName _weaponname)
    (EventDispatchers|UnbindallEventsfromOnComponentBeginOverlap (Variables|Default|GetSphere))
    (Variables|Default|SetOther%20Actor OtherActor)))

(event Custom|Fire
  (Audio|PlaySoundatLocation (Variables|Default|GetWeapon%20Sound) (Transformation|GetActorLocation) "0, 0, 0" 1.0 1.0 0.0 0 0 0 0)
  (Effects|SpawnEmitterAttached (Variables|Default|GetFlash%20Emitter) (Variables|Default|GetSkeletalMesh) "TIP")
  (bind (_location _hitactor _hitcomponent _bonename _impluse) (CallFunction|TraceCamera (Variables|Default|GetWeapon%20Range)))
  (bind (_location1 _hit_actor1 _hit_component1 _bone_name1 _impluse1) (CallFunction|TraceSocket _location _hitactor _hitcomponent _bonename _impluse))
  (Effects|SpawnEmitteratLocation (Variables|Default|GetImpact%20Emitter) _location1)
  (CallFunction|ApplyPhysics _location1 _impluse1 _hit_component1 _bone_name1)
  (Game|Damage|ApplyDamage _hit_actor1 1.5e+02 0 (Variables|Default|GetOther%20Actor)))

(event EventFireON
  (if (Variables|Default|GetAutomatic)
    (Utilities|FlowControl|Gate true) ; enters at Open
    (else
      (Utilities|FlowControl|DoOnce false :!label _label
        (:Completed
          (CallFunction|Fire)
          (Utilities|FlowControl|Delay (Variables|Default|GetFire%20Rate))
          (goto _label Reset))))))

(event EventFireOFF
  (Utilities|FlowControl|Gate true) ; enters at Close
)

(event EventTick
  (params (DeltaSeconds :type Float%20%28single-precision%29))
  (Utilities|FlowControl|Gate true
    (:Exit
      (Utilities|FlowControl|DoOnce false :!label _label
        (:Completed
          (CallFunction|Fire)
          (Utilities|FlowControl|Delay (Variables|Default|GetFire%20Rate))
          (goto _label Reset))))))

(fn ConstructionScript
  (CallFunction|UpdateValues))

(fn OnRepWeaponName
  (CallFunction|UpdateValues))

(fn UpdateValues
  (bind _returnvalue (Utilities|GetDataTableRow "/Game/Inventory/Categories/Weapons/Weapon_Table.Weapon_Table" (Variables|Default|GetWeaponName))
    (:then
      (bind _returnvalue_2 (Utilities|LoadAssetBlocking (.Mesh (Utilities|Struct|BreakWeapon_Structure _returnvalue))))
      (bind _asskeletal_mesh (Utilities|Casting|CastToSkeletalMesh _returnvalue_2))
      (Components|SkeletalMesh|SetSkeletalMeshAsset (Variables|Default|GetSkeletalMesh) _asskeletal_mesh)
      (Variables|Default|SetAutomatic (.Automatic (Utilities|Struct|BreakWeapon_Structure _returnvalue)))
      (Variables|Default|SetFire%20Rate (.FireRate (Utilities|Struct|BreakWeapon_Structure _returnvalue)))
      (bind _returnvalue_3 (Utilities|LoadAssetBlocking (.WeaponSound (Utilities|Struct|BreakWeapon_Structure _returnvalue))))
      (bind _assound_base (Utilities|Casting|CastToSoundBase _returnvalue_3))
      (Variables|Default|SetWeapon%20Sound _assound_base)
      (bind _returnvalue_4 (Utilities|LoadAssetBlocking (.FlashEmitter (Utilities|Struct|BreakWeapon_Structure _returnvalue))))
      (bind _asparticle_system (Utilities|Casting|CastToParticleSystem _returnvalue_4))
      (Variables|Default|SetFlash%20Emitter _asparticle_system)
      (Variables|Default|SetWeapon%20Range (.Range (Utilities|Struct|BreakWeapon_Structure _returnvalue)))
      (bind _returnvalue_5 (Utilities|LoadAssetBlocking (.ImpactEmitter (Utilities|Struct|BreakWeapon_Structure _returnvalue))))
      (bind _asparticle_system_2 (Utilities|Casting|CastToParticleSystem _returnvalue_5))
      (Variables|Default|SetImpact%20Emitter _asparticle_system_2))))

(fn TraceCamera
  (params (Weapon%20Range :type Float%20%28double-precision%29))
  (bind (_world_location _forwards_vector) (Class|BPIInteract|GetCamera(Message) (Variables|Default|GetOther%20Actor)))
  (bind _outhit (Collision|LineTraceByChannel _world_location (+ _world_location (* _forwards_vector Weapon%20Range)) "TraceTypeQuery2" false (Utilities|Array|MakeArray (Variables|Default|GetOther%20Actor)) "None" true "(R=1.000000,G=0.000000,B=0.000000,A=1.000000)" "(R=0.000000,G=1.000000,B=0.000000,A=1.000000)" 1.0))
  (return (select (Utilities|Operators|EqualEqual :A (.Location (Collision|BreakHitResult _outhit))) (.TraceEnd (Collision|BreakHitResult _outhit)) (.Location (Collision|BreakHitResult _outhit))) (.HitActor (Collision|BreakHitResult _outhit)) (.HitComponent (Collision|BreakHitResult _outhit)) (.BoneName (Collision|BreakHitResult _outhit)) (* _forwards_vector Weapon%20Range)))

(fn TraceSocket
  (params (Location :type Vector) (Hit%20Actor :type Actor%20Object%20Reference) (Hit%20Component :type Primitive%20Component%20Object%20Reference) (Bone%20Name :type Name) (Impluse :type Vector))
  (bind _outhit (Collision|LineTraceByChannel (Transformation|GetSocketLocation (Variables|Default|GetSkeletalMesh) "TIP") Location "TraceTypeQuery2" false (Utilities|Array|MakeArray (Variables|Default|GetOther%20Actor)) "ForDuration" true "(R=0.000000,G=0.231939,B=1.000000,A=1.000000)" "(R=0.000000,G=1.000000,B=0.000000,A=1.000000)" 1.0))
  (if (and (Class|KismetMathLibrary|NotEqualExactlyVectorVector "0, 0, 0" (.ImpactPoint (Collision|BreakHitResult _outhit))) (!= Hit%20Component (.HitComponent (Collision|BreakHitResult _outhit))))
    (return (.ImpactPoint (Collision|BreakHitResult _outhit)) (.HitActor (Collision|BreakHitResult _outhit)) (.HitComponent (Collision|BreakHitResult _outhit)) (.BoneName (Collision|BreakHitResult _outhit)) Impluse)
    (else
      (return Location Hit%20Actor Hit%20Component Bone%20Name Impluse))))

(fn ApplyPhysics
  (params (Location :type Vector) (Impulse :type Vector) (Hit%20Component :type Primitive%20Component%20Object%20Reference) (Bone%20Name :type Name))
  (Utilities|IsValid Hit%20Component
    (:Is%20Valid
      (if (Physics|IsSimulatingPhysics Hit%20Component Bone%20Name)
        (Physics|AddImpulseatLocation Hit%20Component (* Impulse 2.0) Location Bone%20Name)))))