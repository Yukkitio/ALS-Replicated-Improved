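; Weapon inventory component that holds owned weapons in a name-keyed map and tracks the active one.
; Give looks up the weapon in Weapon_Table and adds its row to the map, or for an owned weapon sets Ammo on the Find result to the row's value, without summing.
; CycleUp and CycleDown step through the map keys via next/previous array helpers, updating ActiveWeapon and returning its data.
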(fn Give
  (params (WeaponName :type Name))
  (bind _weapons (Variables|Default|GetWeapons))
  (bind (_value _returnvalue) (Utilities|Map|Find _weapons WeaponName))
  (Utilities|FlowControl|Sequence
    (:then_0
      ;[0 0 0] Validate
      (bind _returnvalue_2 (Utilities|GetDataTableRow "/Game/Inventory/Categories/Weapons/Weapon_Table.Weapon_Table" WeaponName)
        (:then
          (Variables|Default|SetOut%20Row _returnvalue_2))
        (:RowNotFound
          (Variables|Default|SetOut%20Row "")
          (return))))
    (:then_1
      ;[0 0 0] Stack Ammo
      (if _returnvalue
        (Utilities|Struct|SetmembersinWeapon_Structure _value (.Ammo (Utilities|Struct|BreakWeapon_Structure (Variables|Default|GetOut%20Row))))
        (return)))
    (:then_2
      ;[0 0 0] Add
      (Utilities|Map|Add (Variables|Default|GetWeapons) WeaponName (Variables|Default|GetOut%20Row))
      (return))))

(fn CycleUp
  (bind _keys (Utilities|Map|Keys (Variables|Default|GetWeapons)))
  (bind _newarrayitem (Utilities|MLGetNextArrayItem _keys (Variables|Default|GetActiveWeapon)))
  (if (.ReturnValue (Utilities|Map|Find (Variables|Default|GetWeapons) _newarrayitem))
    (Variables|Default|SetActiveWeapon _newarrayitem)
    (return (.Value (Utilities|Map|Find (Variables|Default|GetWeapons) _newarrayitem)))
    (else
      (return ""))))

(fn CycleDown
  (bind _keys (Utilities|Map|Keys (Variables|Default|GetWeapons)))
  (bind _newarrayitem (Utilities|MLGetPreviousArrayItem _keys (Variables|Default|GetActiveWeapon)))
  (if (.ReturnValue (Utilities|Map|Find (Variables|Default|GetWeapons) _newarrayitem))
    (Variables|Default|SetActiveWeapon _newarrayitem)
    (return (.Value (Utilities|Map|Find (Variables|Default|GetWeapons) _newarrayitem)))
    (else
      (return ""))))