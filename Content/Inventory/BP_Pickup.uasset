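; BP_Pickup is an inventory pickup actor for items identified by category and name, with weapon handling shown.
; Its construction script switches on category, looks up the name in Weapon_Table and synchronously loads that row's skeletal mesh for display.
; On sphere overlap, it sends PickupWeaponMessage with the item name to actors implementing BPI_Interact.
; The pickup destroys itself only when that call returns true.
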(event OnComponentBeginOverlap(Sphere)
  (params (OverlappedComponent :type Primitive%20Component%20Object%20Reference) (OtherActor :type Actor%20Object%20Reference) (OtherComp :type Primitive%20Component%20Object%20Reference) (OtherBodyIndex :type Integer) (bFromSweep :type Boolean) (SweepResult :type Hit%20Result%20Structure%20%28by%20ref%29))
  (if (Utilities|DoesObjectImplementInterface OtherActor "/Game/Inventory/BPI_Interact.BPI_Interact_C")
    (switch Utilities|FlowControl|Switch|SwitchonItemCategories (Variables|Default|GetItemCategory)
      (:NewEnumerator0
        (bind _succes (Class|BPIInteract|PickupWeapon(Message) OtherActor (Variables|Default|GetItemName)))
        (if _succes
          (Actor|DestroyActor))))))

(event EventBeginPlay)

(event Collision|EventActorBeginOverlap
  (params (OtherActor :type Actor%20Object%20Reference)))

(event EventTick
  (params (DeltaSeconds :type Float%20%28single-precision%29)))

(fn ConstructionScript
  (switch Utilities|FlowControl|Switch|SwitchonItemCategories (Variables|Default|GetItemCategory)
    (:NewEnumerator0
      (bind _returnvalue (Utilities|GetDataTableRow "/Game/Inventory/Categories/Weapons/Weapon_Table.Weapon_Table" (Variables|Default|GetItemName))
        (:then
          (bind _returnvalue_2 (Utilities|LoadAssetBlocking (.Mesh (Utilities|Struct|BreakWeapon_Structure _returnvalue))))
          (bind _asskeletal_mesh (Utilities|Casting|CastToSkeletalMesh _returnvalue_2))
          (Components|SkeletalMesh|SetSkeletalMeshAsset (Variables|Default|GetSkeletalMesh) _asskeletal_mesh))))))